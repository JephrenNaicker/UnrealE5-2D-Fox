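; Ladder prop that lets player 0's character climb upward while W is held.
; Tick compares X and Z offsets to the character, updating OnLadder only within a narrow height band, and prints debug values.
; Both proximity branches enable input on the actor.
; W switches movement to Flying and adds upward input in a 0.2-second Delay loop, restoring Walking when the loop finds either condition false.
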(event `self.ReceiveTick`
  (params (DeltaSeconds :type "Float (single-precision)"))
  (bind (_returnvalue_x _returnvalue_y _returnvalue_z) (`KismetMathLibrary.BreakVector` (`self.K2_GetActorLocation`)))
  (bind _returnvalue (`GameplayStatics.GetPlayerController` 0))
  (bind (_returnvalue_x_2 _returnvalue_y_2 _returnvalue_z_2) (`KismetMathLibrary.BreakVector` (`self.K2_GetActorLocation` (`GameplayStatics.GetPlayerCharacter` 0))))
  (`|ExecutionSequence`
    (:`then_0`
      (set `self.distance` (- _returnvalue_x _returnvalue_x_2)))
    (:`then_1`
      (set `self.height` (- _returnvalue_z _returnvalue_z_2)))
    (:`then_2`
      (if (`KismetMathLibrary.InRange_FloatFloat` (`self.height`) -5.0 5.0)
        (if (`KismetMathLibrary.InRange_FloatFloat` (`self.distance`) -15.0 15.0)
          (set `self.onLadder` true)
          (`self.EnableInput` _returnvalue)
          (else
            (set `self.onLadder` false)
            (`self.EnableInput` _returnvalue)))))
    (:`then_3`
      (`KismetSystemLibrary.PrintString` (`KismetStringLibrary.Conv_BoolToString` (`self.onLadder`)) true true (struct :`R` 0.032179 :`G` 1.0 :`B` 0.020612 :`A` 1.0) 1.0))
    (:`then_4`
      (`KismetSystemLibrary.PrintString` (`KismetStringLibrary.Conv_DoubleToString` (`self.height`)) true true (struct :`G` 0.66 :`B` 1.0 :`A` 1.0) 1.0))))

(event `Key|W`
  (params (Key :type "Key Structure"))
  (bind _returnvalue (`GameplayStatics.GetPlayerPawn` 0))
  (:`Pressed`
    (if (`self.onLadder`) :!label _label
      (if (`PlayerController.IsInputKeyDown` (`GameplayStatics.GetPlayerController` 0) "W")
        (`CharacterMovementComponent.SetMovementMode` (`Character.CharacterMovement` (`GameplayStatics.GetPlayerCharacter` 0)) "MOVE_Flying" 0)
        (`Pawn.AddMovementInput` _returnvalue (`self.GetActorUpVector` _returnvalue) (`self.climbSpead`) false)
        (if (`self.onLadder`)
          (`KismetSystemLibrary.Delay` 0.2)
          (goto _label)
          (else
            _))))
    (`CharacterMovementComponent.SetMovementMode` (`Character.CharacterMovement` (`GameplayStatics.GetPlayerCharacter` 0)) "MOVE_Walking" 0)))

(fn `UserConstructionScript`)