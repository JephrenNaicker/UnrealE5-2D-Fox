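; Cherry pickup for a 2D side-scroller that awards cherry points when the player touches it.
; A sphere overlap, gated by a DoOnce, checks for BP_Player and tells the GM_SliderScoller2D game mode to add points.
; It plays a pickup sound, swaps the flipbook to a feedback animation, then destroys itself after a short delay.
; The DoOnce precedes the player check, so any first overlapping actor consumes it.
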(event `self.Sphere.OnComponentBeginOverlap`
  (params (OverlappedComponent :type "PrimitiveComponent Object Reference") (OtherActor :type "Actor Object Reference") (OtherComp :type "PrimitiveComponent Object Reference") (OtherBodyIndex :type Integer) (bFromSweep :type Boolean) (SweepResult :type "HitResult Structure (by ref)"))
  (`/Engine/EditorBlueprintResources/StandardMacros.DoOnce` false
    (:`Completed`
      (cast `/Game/Blueprint/BP_Player` OtherActor)
      (bind _asgm_slider_scoller_2d (cast `/Game/Blueprint/GM_SliderScoller2D` (`GameplayStatics.GetGameMode`)))
      (`/Game/Blueprint/GM_SliderScoller2D.AddCherryPoints` _asgm_slider_scoller_2d)
      (`GameplayStatics.PlaySound2D` "/Game/Audio/PickUp/Cherry/CherryPickCue.CherryPickCue" 1.0 1.0 0.0 null null)
      (`PaperFlipbookComponent.SetFlipbook` (`self.CherryFlipBook`) "/Game/PNG/sprites/item-feedback/item-feedback.item-feedback")
      (`KismetSystemLibrary.Delay` 1.0)
      (`self.K2_DestroyActor` self))))

(fn `UserConstructionScript`)