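; BP_Player is a 2D side-scrolling player character that moves along the X axis and jumps from input.
; Each tick it turns the control rotation to face the sign of horizontal velocity and picks the sprite's idle, run, jump or falling flipbook.
; Airborne animation relies on an InAir flag, set on jump press and cleared 0.2 seconds after release, rather than vertical velocity.
; UpdateAnimation is empty; GetZValuesTest does that work.
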(event `self.ReceiveTick`
  (params (DeltaSeconds :type "Float (single-precision)"))
  (`self.UpdateAnimation`)
  (`self.UpdateControllRotation`)
  (`self.Get Z values Test`))

(event `InputAxis|MoveRight`
  (params (AxisValue :type "Float (single-precision)"))
  ;[1 1 1] KeyBoard Input
  (`self.AddMovementInput` (1.0 0.0 0.0) AxisValue))

(event `InputAction|Jump`
  (params (Key :type "Key Structure"))
  ;[1 1 1] KeyBoard Input
  (:`Pressed`
    (`self.Jump`)
    (set `self.inAir` true))
  (:`Released`
    (`self.StopJumping`)
    (`KismetSystemLibrary.Delay` 0.2)
    (set `self.inAir` false)))

(event `UpdateAnimation`
  ;[1 1 1] Player Moment
)

(event `UpdateControllRotation`
  ;[1 1 1] Player Rotator
  (`/Engine/EditorBlueprintResources/StandardMacros.IsValid` (`self.GetController`)
    (:`Is Valid`
      (`/Engine/EditorBlueprintResources/StandardMacros.CompareFloat` (`KismetMathLibrary.BreakVector3f` (`MovementComponent.Velocity` (`self.CharacterMovement`)))
        (:`>`
          (`Controller.SetControlRotation` (`self.GetController`) (`KismetMathLibrary.MakeRotator` 0.0)))
        (:`<`
          (`Controller.SetControlRotation` (`self.GetController`) (`KismetMathLibrary.MakeRotator` 0.0 0.0 180.0)))))))

(event `Get Z values Test`
  ;[1 1 1] Testing Play Ground
  (if (`NavMovementComponent.IsMovingOnGround` (`self.GetMovementComponent`))
    (`PaperFlipbookComponent.SetFlipbook` (`self.Sprite`) (select `bool` (> (`KismetMathLibrary.VSize` (`MovementComponent.Velocity` (`self.CharacterMovement`))) 0.0) :`false` "/Game/PNG/sprites/player/idle/player-idle.player-idle" :`true` "/Game/PNG/sprites/player/run/player-run.player-run" :!type "PaperFlipbook Object Reference"))
    (elif (`self.inAir`)
      (`PaperFlipbookComponent.SetFlipbook` (`self.Sprite`) "/Game/PNG/sprites/player/jump/player-jump.player-jump")
      (else
        (`PaperFlipbookComponent.SetFlipbook` (`self.Sprite`) "/Game/PNG/sprites/player/jump/player-falling.player-falling")))))

(fn `UserConstructionScript`)